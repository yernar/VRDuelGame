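; BP_Hexagon is a hexagon mesh actor that shifts vertically when hit by an object on a custom collision channel or triggered through CustomHit.
; Each trigger checks its height: above world Z zero, one timeline lowers it from its stored position, stopping at zero; otherwise another timeline applies a vertical offset curve.
; A DoOnce gate ignores further hits until the active timeline finishes.
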(event OnComponentHit(StaticMesh)
  (params (HitComponent :type Primitive%20Component%20Object%20Reference) (OtherActor :type Actor%20Object%20Reference) (OtherComp :type Primitive%20Component%20Object%20Reference) (NormalImpulse :type Vector :default "0, 0, 0") (Hit :type Hit%20Result%20Structure%20%28by%20ref%29))
  (bind _defaultsceneroot (Variables|Default|GetDefaultSceneRoot))
  (bind _defaultsceneroot_2 (Variables|Default|GetDefaultSceneRoot))
  (bind _returnvalue (Transformation|GetWorldLocation _defaultsceneroot_2))
  (if (Utilities|Enum|Equal(Enum) (Collision|GetCollisionObjectType OtherComp) "ECC_GameTraceChannel1")
    (Utilities|FlowControl|DoOnce false :!label _label
      (:Completed
        (Variables|Default|SetStartPos _returnvalue)
        (if (> (.Z (Math|Vector|BreakVector _returnvalue)) 0.0)
          (Utilities|FlowControl|Sequence
            (:then_0
              (bind _new_location (Timeline|Timeline_1 SetNewTime)
                (:Update
                  (if (<= (+ (.z (Variables|Default|GetStartPos)) (* _new_location -5.0)) 0.0)
                    (Transformation|SetWorldLocation _defaultsceneroot (Math|Vector|MakeVector (.x (Math|Vector|MakeVector (.x (Variables|Default|GetStartPos)) (.y (Variables|Default|GetStartPos)) (+ (.z (Variables|Default|GetStartPos)) (* _new_location -5.0)))) (.y (Math|Vector|MakeVector (.x (Variables|Default|GetStartPos)) (.y (Variables|Default|GetStartPos)) (+ (.z (Variables|Default|GetStartPos)) (* _new_location -5.0)))) 0.0) false false)
                    (else
                      (Transformation|SetWorldLocation _defaultsceneroot (Math|Vector|MakeVector (.x (Math|Vector|MakeVector (.x (Variables|Default|GetStartPos)) (.y (Variables|Default|GetStartPos)) (+ (.z (Variables|Default|GetStartPos)) (* _new_location -5.0)))) (.y (Math|Vector|MakeVector (.x (Variables|Default|GetStartPos)) (.y (Variables|Default|GetStartPos)) (+ (.z (Variables|Default|GetStartPos)) (* _new_location -5.0)))) (.z (Math|Vector|MakeVector (.x (Variables|Default|GetStartPos)) (.y (Variables|Default|GetStartPos)) (+ (.z (Variables|Default|GetStartPos)) (* _new_location -5.0))))) false false))))
                (:Finished
                  (goto _label Reset))))
            (:then_1
              (Timeline|Timeline_1 Play)))
          (else
            (Utilities|FlowControl|Sequence
              (:then_0
                (bind _newtrack_0 (Timeline|Timeline_0 SetNewTime)
                  (:Update
                    (Transformation|SetWorldLocation (Variables|Default|GetDefaultSceneRoot) (Math|Vector|MakeVector (.x (Variables|Default|GetStartPos)) (.y (Variables|Default|GetStartPos)) (+ (.z (Variables|Default|GetStartPos)) _newtrack_0)) false false))
                  (:Finished
                    (goto _label Reset))))
              (:then_1
                (Timeline|Timeline_0 Play)))))))))

(event Custom|CustomHit
  (bind _defaultsceneroot (Variables|Default|GetDefaultSceneRoot))
  (bind _defaultsceneroot_2 (Variables|Default|GetDefaultSceneRoot))
  (bind _returnvalue (Transformation|GetWorldLocation _defaultsceneroot_2))
  (Utilities|FlowControl|DoOnce false :!label _label
    (:Completed
      (Variables|Default|SetStartPos _returnvalue)
      (if (> (.Z (Math|Vector|BreakVector _returnvalue)) 0.0)
        (Utilities|FlowControl|Sequence
          (:then_0
            (bind _new_location (Timeline|Timeline_1 SetNewTime)
              (:Update
                (if (<= (+ (.z (Variables|Default|GetStartPos)) (* _new_location -5.0)) 0.0)
                  (Transformation|SetWorldLocation _defaultsceneroot (Math|Vector|MakeVector (.x (Math|Vector|MakeVector (.x (Variables|Default|GetStartPos)) (.y (Variables|Default|GetStartPos)) (+ (.z (Variables|Default|GetStartPos)) (* _new_location -5.0)))) (.y (Math|Vector|MakeVector (.x (Variables|Default|GetStartPos)) (.y (Variables|Default|GetStartPos)) (+ (.z (Variables|Default|GetStartPos)) (* _new_location -5.0)))) 0.0) false false)
                  (else
                    (Transformation|SetWorldLocation _defaultsceneroot (Math|Vector|MakeVector (.x (Math|Vector|MakeVector (.x (Variables|Default|GetStartPos)) (.y (Variables|Default|GetStartPos)) (+ (.z (Variables|Default|GetStartPos)) (* _new_location -5.0)))) (.y (Math|Vector|MakeVector (.x (Variables|Default|GetStartPos)) (.y (Variables|Default|GetStartPos)) (+ (.z (Variables|Default|GetStartPos)) (* _new_location -5.0)))) (.z (Math|Vector|MakeVector (.x (Variables|Default|GetStartPos)) (.y (Variables|Default|GetStartPos)) (+ (.z (Variables|Default|GetStartPos)) (* _new_location -5.0))))) false false))))
              (:Finished
                (goto _label Reset))))
          (:then_1
            (Timeline|Timeline_1 Play)))
        (else
          (Utilities|FlowControl|Sequence
            (:then_0
              (bind _newtrack_0 (Timeline|Timeline_0 SetNewTime)
                (:Update
                  (Transformation|SetWorldLocation (Variables|Default|GetDefaultSceneRoot) (Math|Vector|MakeVector (.x (Variables|Default|GetStartPos)) (.y (Variables|Default|GetStartPos)) (+ (.z (Variables|Default|GetStartPos)) _newtrack_0)) false false))
                (:Finished
                  (goto _label Reset))))
            (:then_1
              (Timeline|Timeline_0 Play))))))))

(event EventBeginPlay
  (Variables|Default|SetStartPos (Transformation|GetWorldLocation (Variables|Default|GetDefaultSceneRoot))))

(fn ConstructionScript)