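; CH_Spectator is the spectator character for the Duel game, with a screen widget and two hotkey actions.
; On BeginPlay it creates a SceneCapture widget for player controller 0 and adds it to the viewport.
; R opens Map_Main, while F calls RunOnServer, which spawns a scaled-down BP_Pr_RocketGun at player 0's camera manager location and rotation.
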(event Custom|RunOnServer
  (bind _returnvalue (Game|GetPlayerCameraManager 0))
  (bind _rootcomponent (Variables|/Script/Engine.Actor|GetRootComponent _returnvalue))
  (bind _returnvalue_2 (Transformation|GetWorldTransform _rootcomponent))
  (Game|SpawnActorfromClass "/Game/Duel/Blueprints/Weapons/Projectiles/BP_Pr_RocketGun.BP_Pr_RocketGun_C" (Math|Transform|MakeTransform (.location _returnvalue_2) (.rotation _returnvalue_2) "0.300000,0.300000,0.300000") "Undefined" 0 2e+01 4.0 "NewEnumerator1" 0))

(event EventBeginPlay
  (bind _returnvalue (UserInterface|CreateWidget "/Game/Duel/Blueprints/Spectating/SceneCapture.SceneCapture_C" (Game|GetPlayerController 0)))
  (bind _output_get (Variables|Default|SetMyWidget _returnvalue))
  (UserInterface|Viewport|AddtoViewport _output_get 0))

(event Input|KeyboardEvents|R
  (params (Key :type Key%20Structure :default "None"))
  (:Pressed
    (Game|OpenLevel(byName) "Map_Main")))

(event Input|KeyboardEvents|F
  (params (Key :type Key%20Structure :default "None"))
  (:Pressed
    (CallFunction|RunonServer)))

(fn ConstructionScript)