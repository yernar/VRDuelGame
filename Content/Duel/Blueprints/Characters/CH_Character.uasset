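; Networked VR duel character that grabs and fires a weapon in each hand and shows hits as colored body parts.
; Input calls server events that sphere-trace for grabbables and message weapons, with platform-specific haptics on firing.
; RepNotifies drive hand animations, body color and health-bar materials, including one on the watch socket.
; Multicast hits recolor the struck bone's material slot, and zero HP drops weapons, refills health and restores color.
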(event Custom|RunOnServer_AddEff
  (params (Color :type E_Color%20Enum%20%28by%20ref%29 :default "NewEnumerator0") (Bone :type Name) (HitActor :type Actor%20Object%20Reference) (HitLocation :type Vector) (VRPVP :type CH%20VR%20Character%20PVP%20Object%20Reference))
  ;[1 1 1] Fire
  ;;[1 1 1] Damage
  (CallFunction|MulticastAddEff Bone Color HitLocation HitActor)
  (bind _ascontr_vr_character_pvp (Utilities|Casting|CastToContr_VrCharacter_PVP (Pawn|GetController VRPVP)))
  (Default|SpawnHitScreen _ascontr_vr_character_pvp (Variables|CH_Character_C|GetEmitterRoot VRPVP)))

(event Custom|RunOnServer_FireR
  (params (AnimRH :type Anim%20Right%20Hand%20Object%20Reference))
  ;[1 1 1] Fire
  ;;[1 1 1] Rep
  (bind _shoot (Class|IntWeapon|FunFire(Message) (Variables|Right_Hand|GetRightHand_CurrentWeapon) (Variables|Variable|GetColor)))
  (Variables|RightHand|SetShootR _shoot))

(event Custom|RunOnServer_FireL
  (params (AnimLH :type Anim%20Right%20Hand%20Object%20Reference))
  ;[1 1 1] Fire
  ;;[1 1 1] Rep
  (bind _shoot (Class|IntWeapon|FunFire(Message) (Variables|LeftHand|GetLeftHand_CurrentWeapon) (Variables|Variable|GetColor)))
  (Variables|LeftHand|SetShootL _shoot))

(event Custom|Multicast_AddEff
  (params (Bone :type Name) (Color :type E_Color%20Enum%20%28by%20ref%29 :default "NewEnumerator0") (HitLocation :type Vector) (HitActor :type Actor%20Object%20Reference))
  ;[1 1 1] Fire
  ;;[1 1 1] Damage
  (Color|FunSetBoneColor Bone Color)
  (Effects|SpawnEmitteratLocation "/Game/ComicConDuel/Particles/P_Hit.P_Hit" HitLocation (Transformation|GetActorRotation HitActor)))

(event Custom|RunOnServer_StopFireL
  ;[1 1 1] Fire
  ;;[1 1 1] Rep
  (Class|IntWeapon|FunStopFire(Message) (Variables|LeftHand|GetLeftHand_CurrentWeapon))
  (Variables|LeftHand|SetShootL false))

(event Custom|RunOnServer_StopFireR
  ;[1 1 1] Fire
  ;;[1 1 1] Rep
  (Class|IntWeapon|FunStopFire(Message) (Variables|Right_Hand|GetRightHand_CurrentWeapon))
  (Variables|RightHand|SetShootR false))

(event Custom|MulticastSetColor
  ;[1 1 1] Fire
  ;;[1 1 1] Rep
  (Color|FunSetColor (Variables|Variable|GetColor)))

(event Game|Damage|EventAnyDamage
  (params (Damage :type Float%20%28single-precision%29) (DamageType :type Damage%20Type%20Object%20Reference) (InstigatedBy :type Controller%20Object%20Reference) (DamageCauser :type Actor%20Object%20Reference))
  ;[1 1 1] Fire
  ;;[1 1 1] Damage
  (Damage|FunApplyDamage Damage))

(event EventBeginPlay
  (|CallParentFunction)
  (CallFunction|FunInitialization)
  (Transformation|AttachComponentToComponent (Variables|Default|GetHPBar2) (Variables|Default|GetSkeletalMesh) "Watch" "SnapToTarget" "SnapToTarget" "KeepWorld" true))

(event Input|ActionEvents|InputActionFire_Right
  (params (Key :type Key%20Structure :default "None"))
  (bind _righthand_anim (Variables|Right_Hand|GetRightHand_Anim))
  ;[1 1 1] Fire
  (:Pressed
    (if (and (Variables|Right_Hand|GetRightHand_IsValid_Weapon) (Variables|Variable|GetIsEnabledOpposite))
      (Utilities|MacroCanShoot "Right" :!label _label
        (:PressedOut
          (CallFunction|RunonServerFireR _righthand_anim))
        (:ReleasedOut
          (CallFunction|RunonServerStopFireR)))))
  (:Released
    (Variables|/Game/ComicConDuel/Character/Hands/Anim_RightHand.Anim_RightHand_C|SetifTriggerPressed _righthand_anim false)
    (goto _label NewParam)))

(event Input|ActionEvents|InputActionFire_Left
  (params (Key :type Key%20Structure :default "None"))
  (bind _lefthand_anim (Variables|LeftHand|GetLeftHand_Anim))
  ;[1 1 1] Fire
  (:Pressed
    (if (and (Variables|LeftHand|GetLeftHand_IsValid_Weapon) (Variables|Variable|GetIsEnabledOpposite))
      (Utilities|MacroCanShoot "Left" :!label _label
        (:PressedOut
          (CallFunction|RunonServerFireL _lefthand_anim))
        (:ReleasedOut
          (CallFunction|RunonServerStopFireL)))))
  (:Released
    (Variables|/Game/ComicConDuel/Character/Hands/Anim_RightHand.Anim_RightHand_C|SetifTriggerPressed _lefthand_anim false)
    (goto _label NewParam)))

(event Custom|RunOnServer_StartGrabR
  (params (hand :type Scene%20Component%20Object%20Reference))
  ;[1 1 1] Grab Rep
  (bind (_weapon _took _weaponname) (Color|FunStartGrab hand))
  (Variables|Right_Hand|SetRightHand_CurrentWeapon _weapon)
  (Variables|RightHand|SetRightHand_WeaponName _weaponname)
  (Variables|Right_Hand|SetRightHand_IsValid_Weapon _took))

(event Custom|RunOnServer_StopGrabR
  ;[1 1 1] Grab Rep
  ;;[1 1 1] StopGrab
  (Variables|RightHand|SetRightHand_WeaponName "NewEnumerator2")
  (if (Variables|Right_Hand|GetRightHand_IsValid_Weapon)
    (Class|IntWeapon|FunStopGrab(Message) (Variables|Right_Hand|GetRightHand_CurrentWeapon))
    (Variables|Right_Hand|SetRightHand_IsValid_Weapon false)
    (Variables|Right_Hand|SetRightHand_CurrentWeapon 0)))

(event Custom|RunOnServer_StartGrabL
  (params (hand :type Scene%20Component%20Object%20Reference))
  ;[1 1 1] Grab Rep
  (bind (_weapon _took _weaponname) (Color|FunStartGrab hand))
  (Variables|LeftHand|SetLeftHand_CurrentWeapon _weapon)
  (Variables|LeftHand|SetLeftHand_WeaponName _weaponname)
  (Variables|LeftHand|SetLeftHand_IsValid_Weapon _took))

(event Custom|RunOnServer_StopGrabL
  ;[1 1 1] Grab Rep
  ;;[1 1 1] StopGrab
  (Variables|LeftHand|SetLeftHand_WeaponName "NewEnumerator2")
  (if (Variables|LeftHand|GetLeftHand_IsValid_Weapon)
    (Class|IntWeapon|FunStopGrab(Message) (Variables|LeftHand|GetLeftHand_CurrentWeapon))
    (Variables|LeftHand|SetLeftHand_IsValid_Weapon false)
    (Variables|LeftHand|SetLeftHand_CurrentWeapon 0)))

(event Input|ActionEvents|InputActionGrab_Left
  (params (Key :type Key%20Structure))
  ;[1 1 1] Grab Rep
  ;;[1 1 1] start Grab
  (:Pressed
    (CallFunction|RunonServerStartGrabL (Variables|Default|GetHand_L)))
  (:Released
    (CallFunction|RunonServerStopGrabL)))

(event Input|ActionEvents|InputActionGrab_Right
  (params (Key :type Key%20Structure))
  ;[1 1 1] Grab Rep
  ;;[1 1 1] start Grab
  (:Pressed
    (CallFunction|RunonServerStartGrabR (Variables|Default|GetHand_R)))
  (:Released
    (CallFunction|RunonServerStopGrabR)))

(fn ConstructionScript
  (bind _matinstance_hpbar (Variables|Default|GetMatInstance_HPBar))
  (|CallParentFunction)
  (bind _returnvalue (Rendering|Material|CreateDynamicMaterialInstance (Variables|Default|GetHPBar1) 0 "/Game/ComicConDuel/Particles/M_HandUI_Inst.M_HandUI_Inst" "None" :!class /Script/Engine.PrimitiveComponent))
  (Utilities|Array|Add _matinstance_hpbar _returnvalue)
  (bind _returnvalue_2 (Rendering|Material|CreateDynamicMaterialInstance (Variables|Default|GetHPBar2) 0 "/Game/ComicConDuel/Particles/M_HandUI_Inst.M_HandUI_Inst" "None" :!class /Script/Engine.PrimitiveComponent))
  (Utilities|Array|Add _matinstance_hpbar _returnvalue_2)
  (bind _returnvalue_3 (Rendering|Material|CreateDynamicMaterialInstance (Variables|Default|GetHPBar3) 0 "/Game/ComicConDuel/Particles/M_HandUI_Inst.M_HandUI_Inst" "None" :!class /Script/Engine.PrimitiveComponent))
  (Utilities|Array|Add _matinstance_hpbar _returnvalue_3))

(fn OnRepHP
  (for _array_element (Variables|Default|GetMatInstance_HPBar)
    (Rendering|Material|SetScalarParameterValue _array_element "Health" (/ (Variables|Variable|GetHP) 1e+02) :!class /Script/Engine.MaterialInstanceDynamic))
  (Damage|OnHPUpdate)
  (if (<= (Variables|Variable|GetHP) 0.0)
    (Damage|FunDeath)))

(fn OnRepColor
  (Color|FunSetColor (Variables|Variable|GetColor)))

(fn FunStartGrab
  (params (hand :type Scene%20Component%20Object%20Reference))
  (bind _returnvalue (Transformation|GetWorldLocation hand))
  (bind _outhits (Collision|MultiSphereTraceForObjects _returnvalue (+ _returnvalue "0,1.000000, 0") 2e+01 (Utilities|Array|MakeArray "ObjectTypeQuery8") false 0 "None"))
  (if (== (Utilities|Array|Length _outhits) 0)
    (return 0 false "NewEnumerator3" 0)
    (else
      (bind (_took _weaponname) (Class|IntWeapon|FunGrab(Message) (.HitActor (Collision|BreakHitResult (Utilities|Array|Get(acopy) _outhits))) hand))
      (return (.HitActor (Collision|BreakHitResult (Utilities|Array|Get(acopy) _outhits))) _took _weaponname 0))))

(fn FunSetColor
  (params (Color :type E_Color%20Enum%20%28by%20ref%29 :default "NewEnumerator0"))
  (bind _colormap (Variables|Variable|GetColorMap))
  (bind _value (Utilities|Map|Find _colormap Color))
  (Rendering|Material|SetMaterial (Variables|Default|GetHand_L) 0 _value)
  (Rendering|Material|SetMaterial (Variables|Default|GetHand_R) 0 _value)
  (for _index (range 0 7)
    (Rendering|Material|SetMaterial (Variables|Default|GetSkeletalMesh) _index _value)))

(fn FunSetBoneColor
  (params (Bone :type Name) (Color :type E_Color%20Enum%20%28by%20ref%29 :default "NewEnumerator0"))
  (bind _returnvalue (Utilities|String|ToString(Name) Bone))
  (bind _bones_array (Variables|Default|GetBones%20array))
  (bind _colormap (Variables|Variable|GetColorMap))
  (bind _returnvalue_2 (Utilities|Array|FindItem _bones_array _returnvalue))
  (bind _value (Utilities|Map|Find _colormap Color))
  (if (!= _returnvalue_2 -1)
    (Rendering|Material|SetMaterial (Variables|Default|GetSkeletalMesh) _returnvalue_2 _value)
    (switch string _returnvalue
      (:LeftForeArm
        (Rendering|Material|SetMaterial (Variables|Default|GetHand_L) 0 _value))
      (:RightForeArm
        (Rendering|Material|SetMaterial (Variables|Default|GetHand_R) 0 _value)))))

(fn FunApplyDamage
  (params (Damage :type Float%20%28single-precision%29))
  (Variables|Variable|SetHP (- (Variables|Variable|GetHP) Damage)))

(fn FunDeath
  (CallFunction|RunonServerStopGrabR)
  (CallFunction|RunonServerStopGrabL)
  (Variables|Variable|SetHP 1e+02)
  (CallFunction|MulticastSetColor))

(fn OnHPUpdate)

(fn OnRepLeftHandWeaponName
  (Variables|/Game/ComicConDuel/Character/Hands/Anim_RightHand.Anim_RightHand_C|SetWeaponName (Variables|LeftHand|GetLeftHand_Anim) (Variables|LeftHand|GetLeftHand_WeaponName)))

(fn OnRepRightHandWeaponName
  (Variables|/Game/ComicConDuel/Character/Hands/Anim_RightHand.Anim_RightHand_C|SetWeaponName (Variables|Right_Hand|GetRightHand_Anim) (Variables|RightHand|GetRightHand_WeaponName)))

(fn FunInitialization
  ;[1 1 1] Init Anim
  (bind _asanim_right_hand (Utilities|Casting|CastToAnim_RightHand (Components|SkeletalMesh|GetAnimInstance (Variables|Default|GetHand_R))))
  (Variables|Right_Hand|SetRightHand_Anim _asanim_right_hand)
  (bind _asanim_right_hand_2 (Utilities|Casting|CastToAnim_RightHand (Components|SkeletalMesh|GetAnimInstance (Variables|Default|GetHand_L))))
  (Variables|LeftHand|SetLeftHand_Anim _asanim_right_hand_2)
  (for _array_element (Variables|Default|GetMatInstance_HPBar)
    (Rendering|Material|SetScalarParameterValue _array_element "Health" (/ (Variables|Variable|GetHP) 1e+02) :!class /Script/Engine.MaterialInstanceDynamic)))

(fn OnRepShootL
  (Variables|/Game/ComicConDuel/Character/Hands/Anim_RightHand.Anim_RightHand_C|SetifTriggerPressed (Variables|LeftHand|GetLeftHand_Anim) (Variables|LeftHand|GetShootL)))

(fn OnRepShootR
  (Variables|/Game/ComicConDuel/Character/Hands/Anim_RightHand.Anim_RightHand_C|SetifTriggerPressed (Variables|Right_Hand|GetRightHand_Anim) (Variables|RightHand|GetShootR)))

(fn GetColor
  (return (Variables|Variable|GetColor)))