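; Player character for the Duel main menu, supporting menu input from VR motion controllers and showing the mouse cursor on Windows.
; Left and right controller triggers press and release left-mouse clicks through their respective widget interaction components, letting each hand operate UI.
; The O key calls CreateDuelCoop on the GI_Main game instance as a keyboard shortcut.
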(event EventBeginPlay
  (|CallParentFunction)
  (Utilities|GetPlatform
    (:Windows
      (Variables|/Script/Engine.PlayerController|SetbShowMouseCursor (Game|GetPlayerController 0) true))))

(event EventTick
  (params (DeltaSeconds :type Float%20%28single-precision%29))
  (|CallParentFunction DeltaSeconds))

(event Input|KeyboardEvents|MotionControllerLeftTrigger
  (params (Key :type Key%20Structure :default "None"))
  (bind _widgetinteraction_l (Variables|Default|GetWidgetInteraction_L))
  (:Pressed
    (Class|WidgetInteractionComponent|PressPointerKey _widgetinteraction_l "LeftMouseButton"))
  (:Released
    (Class|WidgetInteractionComponent|ReleasePointerKey _widgetinteraction_l "LeftMouseButton")))

(event Input|KeyboardEvents|MotionControllerRightTrigger
  (params (Key :type Key%20Structure :default "None"))
  (bind _widgetinteraction_r (Variables|Default|GetWidgetInteraction_R))
  (:Pressed
    (Class|WidgetInteractionComponent|PressPointerKey _widgetinteraction_r "LeftMouseButton"))
  (:Released
    (Class|WidgetInteractionComponent|ReleasePointerKey _widgetinteraction_r "LeftMouseButton")))

(event Input|KeyboardEvents|O
  (params (Key :type Key%20Structure :default "None"))
  (:Pressed
    (bind _asgi_main (Utilities|Casting|CastToGI_Main (Game|GetGameInstance)))
    (Default|CreateDuelCoop _asgi_main)))

(fn ConstructionScript)