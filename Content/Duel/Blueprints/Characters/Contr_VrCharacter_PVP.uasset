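; Contr_VrCharacter_PVP is a Blueprint for the PVP VR character in the Duel game, adding platform detection and a hit effect.
; The construction script caches the platform from the GI_Main game instance, while BeginPlay only calls the parent.
; A separate GetPlatform function maps Windows and Android to enum values.
; SpawnHitScreen attaches the P_Hit_Screen particle emitter to a supplied component.
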(event EventBeginPlay
  (|CallParentFunction))

(fn ConstructionScript
  (bind _asgi_main (Utilities|Casting|CastToGI_Main (Game|GetGameInstance)))
  (bind _platform (Default|GetMyPlatform _asgi_main))
  (Variables|Default|SetPlatform _platform))

(fn GetPlatform
  (Utilities|GetPlatform
    (:Windows
      (return "NewEnumerator0"))
    (:Android
      (return "NewEnumerator1"))))

(fn SpawnHitScreen
  (params (AttachToComponent :type Scene%20Component%20Object%20Reference))
  (Effects|SpawnEmitterAttached "/Game/ComicConDuel/Particles/P_Hit_Screen.P_Hit_Screen" AttachToComponent "None"))