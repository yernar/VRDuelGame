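; VR player character for PvP duels that syncs head and hand motion across the network.
; The local pawn sends tracking to the server each tick, which moves the controllers and sets HeadRot, applied to remote cameras via OnRep.
; Non-local copies spawn an HP actor and, on the server, a spectator camera rendering to a red or blue target.
; Controllers flagged as spectators swap to CH_Spectator; debug keys open Map_Main.
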(event Custom|ServerUpdate
  (params (transf_Head :type Rotator) (transf_ControllerL :type Transform) (transf_ControllerR :type Transform) (SM_Root :type Transform))
  ;[1 1 1] Server Rep
  (Variables|Default|SetHeadRot transf_Head)
  (Transformation|SetWorldTransform (Variables|Default|GetMotionController_L) transf_ControllerL true false)
  (Transformation|SetWorldTransform (Variables|Default|GetMotionController_R) transf_ControllerR true false))

(event EventBeginPlay
  (bind _returnvalue (Pawn|GetController))
  (bind _self self)
  (bind _self_2 self)
  (bind _self_3 self)
  (bind _follow_camera (Variables|Default|GetFollow%20camera))
  (bind _returnvalue_2 (Transformation|GetWorldTransform _follow_camera))
  (|CallParentFunction)
  (Utilities|FlowControl|Sequence
    (:then_0
      ;[1 1 1] todo
      (if (not (Pawn|IsLocallyControlled))
        (bind _returnvalue_3 (Game|SpawnActorfromClass "/Game/Duel/Blueprints/UserInterfaces/BP_UIHP.BP_UIHP_C" (Math|Transform|MakeTransform (.location _returnvalue_2) (.rotation _returnvalue_2) "1.000000,0.150000,0.120000") "AlwaysSpawn" _self _self))
        (Variables|Default|SetActorWidgetRef _returnvalue_3)
        ;[1 1 1] Spectator
        (Networking|SwitchHasAuthority
          (:Authority
            (Utilities|FlowControl|Delay 0.1)
            (if (Utilities|Enum|Equal(Enum) (Variables|Default|GetColor) "NewEnumerator0")
              (bind _returnvalue_4 (Game|SpawnActorfromClass "/Game/Duel/Blueprints/Spectating/BP_Spectator.BP_Spectator_C" (Transformation|GetWorldTransform (Variables|Default|GetFollow%20camera)) "AlwaysSpawn" _self_3 "/Game/Duel/Blueprints/Spectating/RT_Red_SpectatingRender.RT_Red_SpectatingRender" _self_3))
              (Variables|Default|SetSpec _returnvalue_4)
              (else
                (bind _returnvalue_5 (Game|SpawnActorfromClass "/Game/Duel/Blueprints/Spectating/BP_Spectator.BP_Spectator_C" (Transformation|GetWorldTransform (Variables|Default|GetFollow%20camera)) "AlwaysSpawn" _self_2 "/Game/Duel/Blueprints/Spectating/RT_Blue_SpectatingRender.RT_Blue_SpectatingRender" _self_2))
                (Variables|Default|SetSpec _returnvalue_5)))))))
    (:then_1
      ;[1 1 1] destroy&SpawnSpectator
      (bind _ascontr_vr_character_pvp (Utilities|Casting|CastToContr_VrCharacter_PVP _returnvalue))
      (if (Variables|/Game/Duel/Blueprints/Characters/Contr_VrCharacter_PVP.Contr_VrCharacter_PVP_C|GetSpectator _ascontr_vr_character_pvp)
        (bind _returnvalue_6 (Game|SpawnActorfromClass "/Game/Duel/Blueprints/Characters/CH_Spectator.CH_Spectator_C" (Transformation|GetActorTransform) "Undefined" _returnvalue 0))
        (Pawn|UnPossess _ascontr_vr_character_pvp)
        (Pawn|Possess _ascontr_vr_character_pvp _returnvalue_6)
        (Actor|DestroyActor)))))

(event EventEndPlay
  (params (EndPlayReason :type EEndPlayReason%20Enum :default "Destroyed"))
  (|CallParentFunction EndPlayReason)
  (bind _actorwidgetref (Variables|Default|GetActorWidgetRef)
    (:then
      (Actor|DestroyActor _actorwidgetref))
    (:else
      _))
  (bind _spec (Variables|Default|GetSpec)
    (:then
      (Actor|DestroyActor _spec))
    (:else)))

(event EventTick
  (params (DeltaSeconds :type Float%20%28single-precision%29))
  (|CallParentFunction DeltaSeconds)
  ;[1 1 1] Rep
  (if (Pawn|IsLocallyControlled)
    (CallFunction|ServerUpdate (Transformation|GetWorldRotation (Variables|Default|GetFollow%20camera)) (Transformation|GetWorldTransform (Variables|Default|GetMotionController_L)) (Transformation|GetWorldTransform (Variables|Default|GetMotionController_R)) (Transformation|GetWorldTransform (Variables|Default|GetSM_Root)))))

(event Input|KeyboardEvents|MotionControllerRightFaceButton2
  (params (Key :type Key%20Structure :default "None"))
  ;[1 1 1] Debug Only
  (:Pressed
    (Game|OpenLevel(byName) "Map_Main")))

(event Input|KeyboardEvents|R
  (params (Key :type Key%20Structure :default "None"))
  ;[1 1 1] Debug Only
  (:Pressed
    (Game|OpenLevel(byName) "Map_Main")))

(fn ConstructionScript)

(fn OnRepHeadRot
  (if (not (Pawn|IsLocallyControlled))
    (Transformation|SetWorldRotation (Variables|Default|GetFollow%20camera) (Variables|Default|GetHeadRot) false false)))

(fn GetSceneCharacters
  (params (SceneCharacters :type Array%20of%20CH%20VR%20Character%20PVP%20Object%20References))
  (Variables|Default|SetSceneCharacters SceneCharacters)
  (Utilities|Array|RemoveIndex (Variables|Default|GetSceneCharacters) (Utilities|Array|FindItem (Variables|Default|GetSceneCharacters) self)))

(fn SpawnSpectatorCamera
  (bind _self self)
  (Game|SpawnActorfromClass "/Game/Duel/Blueprints/Spectating/BP_Spectator.BP_Spectator_C" (Transformation|GetWorldTransform (Variables|Default|GetFollow%20camera)) "AlwaysSpawn" _self "/Game/Duel/Blueprints/Spectating/RT_Red_SpectatingRender.RT_Red_SpectatingRender" _self))