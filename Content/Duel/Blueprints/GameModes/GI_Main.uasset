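; Game instance for the Duel game that hosts and joins multiplayer sessions.
; Two create events start an online session and open either the co-op or ComicCon duel map as a listen server.
; Joining either uses a direct connection to localhost on Windows or a hardcoded LAN IP elsewhere, or finds sessions and joins the first result.
; A helper maps Windows and Android to a platform enum; an advanced session search is left unwired.
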(event Custom|CreateGame
  (|Session (Game|GetPlayerController 0) 3 false
    (:then
      (Game|OpenLevel(byName) "Map_ComicConDuel" true "listen")
      (Utilities|FlowControl|DoOnce false
        (:Completed
          (Development|ExecuteConsoleCommand "stat fps" 0))))
    (:OnSuccess
      (Development|PrintString "Succest"))
    (:OnFailure
      (Development|PrintString "Fail"))))

(event Custom|ConnectGame
  (if (Utilities|Enum|Equal(Enum) (Game|GetPlatformName) "Windows")
    (Development|ExecuteConsoleCommand "open localhost" 0)
    (else
      (Development|ExecuteConsoleCommand "open 192.168.2.101" 0)))
  (Utilities|FlowControl|DoOnce false
    (:Completed
      (Development|ExecuteConsoleCommand "stat fps" 0))))

(event Custom|FindAndConnect
  (bind _returnvalue (Game|GetPlayerController 0))
  (bind _results (|FindSessions _returnvalue 2 false)
    (:OnSuccess
      (|JoinSession _returnvalue (Utilities|Array|Get(acopy) _results)
        (:OnSuccess
          (Development|PrintString "Success" true true "(R=0.195120,G=1.000000,B=0.000000,A=1.000000)" 4.0))
        (:OnFailure
          (Development|PrintString "Fail" true true "(R=1.000000,G=0.024960,B=0.000000,A=1.000000)" 4.0))))))

(event Custom|CreateDuelCoop
  (|Session 0 3 false
    (:then
      (Game|OpenLevel(byName) "Map_DuelCoop" true "listen")
      (Development|ExecuteConsoleCommand "stat fps" 0))))

(fn GetMyPlatform
  (switch string (Game|GetPlatformName)
    (:Windows
      (return "NewEnumerator0"))
    (:Android
      (return "NewEnumerator1"))))