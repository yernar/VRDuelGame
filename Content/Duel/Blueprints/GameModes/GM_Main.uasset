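; Game mode for VR PvP that assigns joining players to colored spawn points or a spectator spot.
; ChoosePlayerStart claims a free player spawner, but flags the first player as spectator if no headset is connected.
; Pawn spawning copies the spawner's color and registers a new GUID, color and spawner in GS_Main, storing the ID on the controller.
; Logout uses that ID to free the spawner; MustSpectate simply defers to the parent.
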(event EventOnLogout
  (params (ExitingController :type Controller%20Object%20Reference))
  (Development|PrintString "logout")
  (bind _ascontr_vr_character_pvp (Utilities|Casting|CastToContr_VrCharacter_PVP ExitingController))
  (bind _asgs_main (Utilities|Casting|CastToGS_Main (Game|GetGameState)))
  (for _array_element (Variables|/Game/Duel/Blueprints/GameModes/GS_Main.GS_Main_C|Getf_characters _asgs_main)
    (if (== (.Id (Utilities|Struct|BreakF_Character _array_element)) (Variables|/Game/Duel/Blueprints/Characters/Contr_VrCharacter_PVP.Contr_VrCharacter_PVP_C|Getid _ascontr_vr_character_pvp))
      (Variables|/Game/Duel/Blueprints/Characters/PS_PlayersSpawner.PS_PlayersSpawner_C|SetisBusy (.spawner (Utilities|Struct|BreakF_Character _array_element)) false))))

(fn ConstructionScript
  (|CallParentFunction))

(fn ChoosePlayerStart
  (params (Player :type Controller%20Object%20Reference))
  (LocalVariables|SetCurrentController Player)
  (if (or (not (Variables|Default|GetfirstPlayer)) (Class|HeadMountedDisplayFunctionLibrary|IsHeadMountedDisplayConnected))
    ;[1 1 1] set Spawners arr
    (bind _outactors (Actor|GetAllActorsOfClass "/Game/Duel/Blueprints/Characters/PS_PlayersSpawner.PS_PlayersSpawner_C"))
    (Variables|Default|SetSpawners _outactors)
    ;[1 1 1] check spawn is busy
    (for _array_element (Variables|Default|GetSpawners)
      (if (not (Variables|/Game/Duel/Blueprints/Characters/PS_PlayersSpawner.PS_PlayersSpawner_C|GetisBusy _array_element))
        (Variables|Default|SetCurrentSpawner _array_element)
        (Variables|/Game/Duel/Blueprints/Characters/PS_PlayersSpawner.PS_PlayersSpawner_C|SetisBusy _array_element true)
        ;[1 1 1] Return
        (return (Variables|Default|GetCurrentSpawner))))
    (else
      ;[1 1 1] GetSpectatorSpawner
      (Variables|Default|SetFirstPlayer false)
      (bind _ascontr_vr_character_pvp (Utilities|Casting|CastToContr_VrCharacter_PVP (LocalVariables|GetCurrentController))
        (:then
          (Variables|/Game/Duel/Blueprints/Characters/Contr_VrCharacter_PVP.Contr_VrCharacter_PVP_C|SetSpectator _ascontr_vr_character_pvp true))
        (:CastFailed
          _))
      (bind _outactors_2 (Actor|GetAllActorsOfClass "/Game/Duel/Blueprints/Characters/PS_SpectatorSpawner.PS_SpectatorSpawner_C"))
      (return (Utilities|Array|Get(acopy) _outactors_2)))))

(fn MustSpectate
  (params (NewPlayerController :type Player%20Controller%20Object%20Reference))
  (bind _ascontr_vr_character_pvp (Utilities|Casting|CastToContr_VrCharacter_PVP NewPlayerController)
    (:then
      (if (Variables|/Game/Duel/Blueprints/Characters/Contr_VrCharacter_PVP.Contr_VrCharacter_PVP_C|GetSpectator _ascontr_vr_character_pvp)
        (bind _returnvalue (|CallParentFunction NewPlayerController))
        (return _returnvalue)
        (else
          _)))
    (:CastFailed
      _))
  (bind _returnvalue_2 (|CallParentFunction NewPlayerController))
  (return _returnvalue_2))

(fn SpawnDefaultPawnatTransform
  (params (NewPlayer :type Controller%20Object%20Reference) (SpawnTransform :type Transform%20%28by%20ref%29))
  (bind _output_get (LocalVariables|SetController NewPlayer))
  (bind _returnvalue (|CallParentFunction _output_get SpawnTransform))
  (bind _asps_players_spawner (Utilities|Casting|CastToPS_PlayersSpawner (Variables|Default|GetCurrentSpawner))
    (:then
      (LocalVariables|SetPlayerSpawner _asps_players_spawner)
      (bind _asch_vrcharacter_pvp (Utilities|Casting|CastToCH_VRCharacterPVP _returnvalue))
      (LocalVariables|SetCHPVP _asch_vrcharacter_pvp)
      (Variables|/Game/Duel/Blueprints/Characters/CH_Character.CH_Character_C|SetColor (LocalVariables|GetCHPVP) (Variables|/Game/Duel/Blueprints/Characters/PS_PlayersSpawner.PS_PlayersSpawner_C|GetColor (LocalVariables|GetPlayerSpawner)))
      (LocalVariables|SetNewId (Guid|NewGuid))
      (bind _asgs_main (Utilities|Casting|CastToGS_Main (Game|GetGameState)))
      (Utilities|Array|Add (Variables|/Game/Duel/Blueprints/GameModes/GS_Main.GS_Main_C|Getf_characters _asgs_main) (Utilities|Struct|MakeF_Character (LocalVariables|GetNewId) (Variables|/Game/Duel/Blueprints/Characters/PS_PlayersSpawner.PS_PlayersSpawner_C|GetColor (LocalVariables|GetPlayerSpawner)) (LocalVariables|GetPlayerSpawner)))
      (bind _ascontr_vr_character_pvp (Utilities|Casting|CastToContr_VrCharacter_PVP (LocalVariables|GetController)))
      (Variables|/Game/Duel/Blueprints/Characters/Contr_VrCharacter_PVP.Contr_VrCharacter_PVP_C|Setid _ascontr_vr_character_pvp (LocalVariables|GetNewId))
      (return (LocalVariables|GetCHPVP)))
    (:CastFailed
      (return _returnvalue))))