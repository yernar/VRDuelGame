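; Spectator camera actor for a VR PVP duel character that renders a scene capture into a render target.
; BeginPlay caches the owning character and assigns the target; Tick snaps the root to the character's SMRoot location and follow-camera rotation.
; Interpolated free-fly movement, pitch and yaw functions are defined but not called here.
; The function that shows the blue spectating render target on the spectator screen is never run.
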(event EventBeginPlay
  (bind _asch_vrcharacter_pvp (Utilities|Casting|CastToCH_VRCharacterPVP (Components|GetOwner)))
  (Variables|Default|SetCH_Owner _asch_vrcharacter_pvp)
  (Variables|/Script/Engine.SceneCaptureComponent2D|SetTextureTarget (Variables|Default|GetSceneCaptureComponent2D) (Variables|Default|GetTextureRenderTarget)))

(event EventTick
  (params (DeltaSeconds :type Float%20%28single-precision%29))
  (bind _ch_owner (Variables|Default|GetCH_Owner))
  (Transformation|SetWorldTransform (Variables|Default|GetDefaultSceneRoot) (Math|Transform|MakeTransform (.location (Transformation|GetWorldTransform (Variables|/Game/Duel/Blueprints/Characters/ThirdPersonCharacter.ThirdPersonCharacter_C|GetSM_Root _ch_owner))) (Transformation|GetWorldRotation (Variables|/Game/Duel/Blueprints/Characters/ThirdPersonCharacter.ThirdPersonCharacter_C|GetFollow%20camera _ch_owner)) "1,1,1") false false))

(fn ConstructionScript)

(fn CameraPitchRotation
  (bind _output_get (Variables|Default|SetPitchRotationDelta (Math|Interpolation|FInterpTo (Variables|Default|GetPitchRotationDelta) (Input|AxisValues|GetLookUp) (Utilities|Time|GetWorldDeltaSeconds) (Variables|Default|GetInterpolationSpeed))))
  (Transformation|AddRelativeRotation (Variables|Default|GetSceneCaptureComponent2D) (Math|Rotator|MakeRotator 0.0 _output_get 0.0) false false))

(fn CameraYawRotation
  (bind _output_get (Variables|Default|SetYawRotationDelta (Math|Interpolation|FInterpTo (Variables|Default|GetYawRotationDelta) (Input|AxisValues|GetLookRight) (Utilities|Time|GetWorldDeltaSeconds) (Variables|Default|GetInterpolationSpeed))))
  (Class|Actor|AddActorWorldRotation (Math|Rotator|MakeRotator 0.0 0.0 _output_get)))

(fn CameraMovement
  (bind _scenecapturecomponent2d (Variables|Default|GetSceneCaptureComponent2D))
  (bind _output_get (Variables|Default|SetMovementOffset (Math|Interpolation|VInterpTo (Variables|Default|GetMovementOffset) (* (+ (* (Math|Vector|GetForwardVector _scenecapturecomponent2d) (Input|AxisValues|GetMoveForward)) (* (Math|Vector|GetRightVector _scenecapturecomponent2d) (Input|AxisValues|GetMoveRight)) (Math|Vector|MakeVector 0.0 0.0 (Input|AxisValues|GetMoveUp))) (Variables|Default|GetMovementSpeed)) (Utilities|Time|GetWorldDeltaSeconds) (Variables|Default|GetInterpolationSpeed))))
  (Transformation|AddActorWorldOffset _output_get))

(fn SetSpectatorScreen
  (Class|HeadMountedDisplayFunctionLibrary|SetSpectatorScreenMode "Texture")
  (Class|HeadMountedDisplayFunctionLibrary|SetSpectatorScreenTexture "/Game/Duel/Blueprints/Spectating/RT_Blue_SpectatingRender.RT_Blue_SpectatingRender"))