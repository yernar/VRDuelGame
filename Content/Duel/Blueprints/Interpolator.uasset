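; Scene component in Duel that smooths replicated movement by interpolating its world transform on non-authority machines.
; Each tick the authority writes its transform to NetTransform, while others lerp location and rotation toward it over TransitionTime.
; A rep-notify records the update time and current transform as the blend start.
; Scale is captured but never applied, location alpha is not clamped after division, and SmoothDampVector is an empty stub.
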(event EventBeginPlay
  (CallFunction|Init))

(event EventTick
  (params (DeltaSeconds :type Float%20%28single-precision%29))
  (bind _t (CallFunction|GetTimeSinceLastUpdate))
  (bind _transitiontime (Variables|Default|GettransitionTime))
  (bind _returnvalue (/ _t _transitiontime))
  (if (Ability|HasAuthority (Components|GetOwner))
    (Variables|Default|SetnetTransform (Math|Transform|MakeTransform (Transformation|GetWorldLocation) (Transformation|GetWorldRotation) (Transformation|GetWorldScale)))
    (else
      (Transformation|SetWorldLocation (Math|Vector|Lerp(Vector) (.location (Variables|Default|GetlastKnownTransform)) (.location (Variables|Default|GetnetTransform)) _returnvalue) false false)
      (Transformation|SetWorldRotation (Math|Rotator|Lerp(Rotator) (.rotation (Variables|Default|GetlastKnownTransform)) (.rotation (Variables|Default|GetnetTransform)) (Math|Float|Clamp(Float) _returnvalue)) false false))))

(fn SmoothDamp(Vector)
  (params (NewParam :type Vector) (NewParam1 :type Vector) (T :type Float%20%28single-precision%29)))

(fn GetTimeSinceLastUpdate
  (return (Math|Float|Clamp(Float) (- (Utilities|Time|GetRealTimeSeconds) (Variables|Default|GetlastUpdate)))))

(fn OnRepNetLocation
  (Variables|Default|SetlastUpdate (Utilities|Time|GetRealTimeSeconds))
  (Variables|Default|SetlastKnownTransform (Transformation|GetWorldTransform)))

(fn Init
  (bind _output_get (Variables|Default|SetnetTransform (Math|Transform|MakeTransform (Transformation|GetWorldLocation) (Transformation|GetWorldRotation) (Transformation|GetWorldScale))))
  (Variables|Default|SetlastKnownTransform _output_get))