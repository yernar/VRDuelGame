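; Rocket gun projectile for PVP duels that explodes when it leaves play, with the server setting its lifespan.
; On EndPlay, the server sphere-traces around the mesh, triggers a colored effect for each VR character hit and gathers unique characters and hexagons.
; It then damages each character once and calls CustomHit on each hexagon, while clients only spawn the explosion particles.
; The blast trace still has timed debug drawing enabled.
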(event EventEndPlay
  (params (EndPlayReason :type EEndPlayReason%20Enum :default "Destroyed"))
  (|CallParentFunction EndPlayReason)
  (Networking|SwitchHasAuthority
    (:Authority
      (CallFunction|PVPCharacterApplyDamageAuthority))
    (:Remote
      (CallFunction|PVPCharacterApplyDamageClient))))

(event EventBeginPlay
  (Networking|SwitchHasAuthority
    (:Authority
      (Actor|SetLifeSpan (Variables|Default|GetLifeTime)))))

(fn ConstructionScript)

(fn PVPCharacterApplyDamageAuthority
  (bind _staticmesh (Variables|Default|GetStaticMesh))
  (bind _returnvalue (Transformation|GetWorldLocation _staticmesh))
  (bind _outhits (Collision|MultiSphereTraceForObjects _returnvalue (+ _returnvalue "1.000000, 0, 0") 1.8e+02 (Utilities|Array|MakeArray "ObjectTypeQuery3" "ObjectTypeQuery9") false 0 "ForDuration"))
  (for _array_element _outhits
    (bind _asch_vrcharacter_pvp (Utilities|Casting|CastToCH_VRCharacterPVP (.HitActor (Collision|BreakHitResult _array_element)))
      (:then
        (Default|RunonServerAddEff _asch_vrcharacter_pvp (Variables|Default|GetColor) (.HitBoneName (Collision|BreakHitResult _array_element)) (.HitActor (Collision|BreakHitResult _array_element)) (.Location (Collision|BreakHitResult _array_element)) _asch_vrcharacter_pvp)
        (Utilities|Array|AddUnique (Variables|Default|GetDamaged) _asch_vrcharacter_pvp))
      (:CastFailed
        (bind _asbp_hexagon (Utilities|Casting|CastToBP_Hexagon (.HitActor (Collision|BreakHitResult _array_element))))
        (Utilities|Array|AddUnique (Variables|Default|GetHexagons) _asbp_hexagon))))
  (Effects|SpawnEmitteratLocation "/Game/ComicConDuel/Particles/P_Explosion.P_Explosion" (Transformation|GetWorldLocation (Variables|Default|GetStaticMesh)))
  (for _array_element_2 (Variables|Default|GetDamaged)
    (Game|Damage|ApplyDamage _array_element_2 (Variables|Default|GetDamage) 0 0))
  (for _array_element_3 (Variables|Default|GetHexagons)
    (Default|CustomHit _array_element_3)))

(fn PVPCharacterApplyDamageClient
  (Effects|SpawnEmitteratLocation "/Game/ComicConDuel/Particles/P_Explosion.P_Explosion" (Transformation|GetWorldLocation (Variables|Default|GetStaticMesh))))