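; Grabbable gun for VR PvP duels that fires colored projectiles with a muzzle flash, limited by a short cooldown.
; Grabbing rejects an already held gun, otherwise snaps it to the hand socket, disables physics and picks a material from the VR character's color.
; Release detaches it, restores physics and resets animation.
; Net priority rises while held, and the IsFire RepNotify drives the weapon's anim instance.
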(event Custom|SetRecentlyShoot
  (Utilities|FlowControl|Delay 0.35)
  (Variables|Default|SetRecentlyShoot false))

(event EventBeginPlay
  (Variables|Default|SetWeaponAnim (Components|SkeletalMesh|GetAnimInstance (Variables|Default|GetSkeletalMesh))))

(fn ConstructionScript)

(fn OnRepIsFire
  (Class|IntAnimWeapon|FunAnimFire(Message) (Variables|Default|GetWeaponAnim) (Variables|Default|GetIsFire) true))

(fn FunFire
  (params (Color :type E_Color%20Enum :default "NewEnumerator0"))
  (bind _firepoint (Variables|Default|GetFirePoint))
  (bind _returnvalue (Transformation|GetWorldTransform _firepoint))
  (Variables|Default|SetIsFire true)
  (if (Variables|Default|GetRecentlyShoot)
    _
    (else
      (Variables|Default|SetRecentlyShoot true)
      (Game|SpawnActorfromClass "/Game/Duel/Blueprints/Weapons/Projectiles/BP_FirstPersonProjectile.BP_FirstPersonProjectile_C" (Transformation|GetWorldTransform (Variables|Default|GetFirePoint)) "AdjustIfPossibleButAlwaysSpawn" 0 (Variables|Default|GetDamage) (Variables|Default|GetLifeTimeBullet) Color 0)
      (Effects|SpawnEmitteratLocation "/Game/ComicConDuel/Particles/P_Lightning_Muzzle_Flash_5.P_Lightning_Muzzle_Flash_5" (.location _returnvalue) (.rotation _returnvalue))
      (CallFunction|SetRecentlyShoot)))
  (return true))

(fn FunGetAnim
  (return (Variables|Default|GetWeaponAnim)))

(fn FunGrab
  (params (Hand :type Scene%20Component%20Object%20Reference))
  (bind _skeletalmesh (Variables|Default|GetSkeletalMesh))
  (if (Variables|Default|GetisTaken)
    (return false "NewEnumerator3")
    (else
      (Variables|Default|SetisTaken true)
      (Transformation|AttachComponentToComponent (Variables|Debug|GetStaticMeshComponent) Hand "Gun" "SnapToTarget" "SnapToTarget" "KeepWorld" true)
      (Variables|Default|SetNetPriority 3.0)
      (Physics|SetSimulatePhysics (Variables|Debug|GetStaticMeshComponent) false)
      (bind _asch_vrcharacter_pvp (Utilities|Casting|CastToCH_VRCharacterPVP (Components|GetOwner Hand))
        (:then
          (if (Utilities|Enum|Equal(Enum) (Variables|/Game/Duel/Blueprints/Characters/CH_Character.CH_Character_C|GetColor _asch_vrcharacter_pvp) "NewEnumerator0")
            (Rendering|Material|SetMaterial _skeletalmesh 0 "/Game/ComicConDuel/Gun/Pistol/M_GunMM_Inst_4.M_GunMM_Inst_4")
            (else
              (Rendering|Material|SetMaterial _skeletalmesh 0 "/Game/ComicConDuel/Gun/Pistol/M_GunMM_Inst_5.M_GunMM_Inst_5")))
          (return true (Variables|Default|GetWeaponName)))
        (:CastFailed
          (return true (Variables|Default|GetWeaponName)))))))

(fn FunStopFire
  (Variables|Default|SetIsFire false)
  (return false))

(fn FunStopGrab
  (Variables|Default|SetisTaken false)
  (Transformation|DetachFromComponent (Variables|Debug|GetStaticMeshComponent) "KeepWorld" "KeepWorld" "KeepWorld" true)
  (Physics|SetSimulatePhysics (Variables|Debug|GetStaticMeshComponent) true)
  (Class|IntAnimWeapon|FunSetDefaultState(Message) (Variables|Default|GetWeaponAnim))
  (Variables|Default|SetNetPriority 1.0)
  (return false))