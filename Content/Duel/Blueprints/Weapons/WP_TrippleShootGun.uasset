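; Triple-shot gun weapon for the Duel game that can be grabbed and dropped, though its fire and get-anim functions are empty stubs.
; Grabbing an untaken gun snaps its mesh to the hand's Gun socket, disables physics and raises net priority, yet reports Took as false.
; Release detaches it and restores physics and priority.
; Stop-fire and release send messages to the anim instance cached at BeginPlay.
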(event EventBeginPlay
  (Variables|Default|SetWeaponAnim (Components|SkeletalMesh|GetAnimInstance (Variables|Default|GetSkeletalMesh))))

(fn ConstructionScript
  (|CallParentFunction))

(fn FunFire
  (params (Color :type E_Color%20Enum :default "NewEnumerator0")))

(fn FunGetAnim
  (return 0))

(fn FunGrab
  (params (Hand :type Scene%20Component%20Object%20Reference))
  (if (Variables|Default|GetisTaken)
    (return false "NewEnumerator3")
    (else
      (Variables|Default|SetisTaken true)
      (Transformation|AttachComponentToComponent (Variables|Debug|GetStaticMeshComponent) Hand "Gun" "SnapToTarget" "SnapToTarget" "KeepWorld" true)
      (Variables|Default|SetNetPriority 2.0)
      (Physics|SetSimulatePhysics (Variables|Debug|GetStaticMeshComponent) false)
      (return false (Variables|Default|GetWeaponName)))))

(fn FunStopFire
  (Class|IntAnimWeapon|FunAnimFire(Message) (Variables|Default|GetWeaponAnim) false true)
  (return false))

(fn FunStopGrab
  (Variables|Default|SetisTaken false)
  (Transformation|DetachFromComponent (Variables|Debug|GetStaticMeshComponent) "KeepWorld" "KeepWorld" "KeepWorld" true)
  (Physics|SetSimulatePhysics (Variables|Debug|GetStaticMeshComponent) true)
  (Class|IntAnimWeapon|FunSetDefaultState(Message) (Variables|Default|GetWeaponAnim))
  (Variables|Default|SetNetPriority 1.0)
  (return false))