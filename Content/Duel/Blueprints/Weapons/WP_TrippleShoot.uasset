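; Triple-shot weapon for the Duel game that fires small, colored rocket projectiles with a muzzle flash from FirePoint.
; Grabbing snaps the mesh to a hand socket and disables its physics.
; An empty magazine starts a looping timer that reads the held gun's vertical velocity: a fast downward motion refills and enters reloading, a fast upward one ends it.
; The Reloading RepNotify passes that state to the weapon's AnimInstance.
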(event Custom|CustomEvent_0
  (if (Variables|Default|GetIsTaken)
    (bind _returnvalue (Physics|GetPhysicsLinearVelocity (Variables|Default|GetStaticMeshComponent) "None"))
    (if (Variables|Default|GetReloading)
      (if (> (.z _returnvalue) 3e+02)
        (Variables|Default|SetReloading false)
        (Utilities|Time|PauseTimerbyHandle (stale Custom|Reload _returnvalue)))
      (elif (< (.z _returnvalue) -3e+02)
        (Variables|Default|SetReloading true)
        (Variables|Default|SetBullets 3)))))

(event Custom|Reload
  (bind _returnvalue (Utilities|Time|SetTimerbyEvent (delegate Custom|CustomEvent_0) 0.05 true)))

(event EventBeginPlay
  (|CallParentFunction)
  (Variables|Default|SetWeaponAnim (Components|SkeletalMesh|GetAnimInstance (Variables|Default|GetSkeletalMesh))))

(event Collision|EventActorBeginOverlap
  (params (OtherActor :type Actor%20Object%20Reference)))

(event EventTick
  (params (DeltaSeconds :type Float%20%28single-precision%29)))

(fn ConstructionScript
  (|CallParentFunction)
  (Variables|Default|SetWeaponName "NewEnumerator1"))

(fn FunFire
  (params (Color :type E_Color%20Enum :default "NewEnumerator0"))
  (bind _firepoint (Variables|Default|GetFirePoint))
  (bind _firepoint_2 (Variables|Default|GetFirePoint))
  (bind _returnvalue (Transformation|GetWorldTransform _firepoint))
  (bind _returnvalue_2 (Transformation|GetWorldTransform _firepoint_2))
  (if (and (not (Variables|Default|GetReloading)) (> (Variables|Default|GetBullets) 0))
    (Game|SpawnActorfromClass "/Game/Duel/Blueprints/Weapons/Projectiles/BP_Pr_RocketGun.BP_Pr_RocketGun_C" (Math|Transform|MakeTransform (.location _returnvalue) (.rotation _returnvalue) "0.100000,0.100000,0.100000") "AdjustIfPossibleButAlwaysSpawn" 0 (Variables|Default|GetDamage) (Variables|Default|GetLifeTimeBullet) Color 0)
    (Effects|SpawnEmitteratLocation "/Game/ComicConDuel/Particles/P_Lightning_Muzzle_Flash_5.P_Lightning_Muzzle_Flash_5" (.location _returnvalue_2) (.rotation _returnvalue_2))
    (Variables|Default|SetIsFire true)
    (bind _output_get (Variables|Default|SetBullets (- (Variables|Default|GetBullets) 1)))
    (if (<= _output_get 0)
      (CallFunction|Reload)
      (else
        (return true)))
    (else
      (return false))))

(fn FunGrab
  (params (Hand :type Scene%20Component%20Object%20Reference))
  (if (Variables|Default|GetisTaken)
    (return false "NewEnumerator3")
    (else
      (Variables|Default|SetisTaken true)
      (Transformation|AttachComponentToComponent (Variables|Default|GetStaticMeshComponent) Hand "TrippleShootGun" "SnapToTarget" "SnapToTarget" "KeepWorld" true)
      (Variables|Default|SetNetPriority 3.0)
      (Physics|SetSimulatePhysics (Variables|Default|GetStaticMeshComponent) false)
      (return true (Variables|Default|GetWeaponName)))))

(fn OnRepReloading
  (Class|IntAnimWeapon|FunReloading(Message) (Variables|Default|GetWeaponAnim) (Variables|Default|GetReloading)))