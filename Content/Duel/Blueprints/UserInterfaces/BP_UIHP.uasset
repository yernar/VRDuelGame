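; BP_UIHP is a world-space health bar that floats above its owning CH_VRCharacterPVP in the VR duel game.
; On BeginPlay it caches the owning character and the UI_HP widget, then starts a fast looping timer instead of using Tick.
; Each timer pass pushes normalized HP into the widget, moves it above the skeletal mesh, billboards it toward the local camera with zero roll, and requests a redraw.
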(event Custom|CustomTimer
  (bind _returnvalue (Game|GetPlayerController 0))
  (bind _widget (Variables|Default|GetWidget))
  (bind _returnvalue_2 (Transformation|GetWorldLocation _widget))
  (bind _playercameramanager (Variables|/Script/Engine.PlayerController|GetPlayerCameraManager _returnvalue))
  (bind _returnvalue_3 (Camera|GetCameraLocation _playercameramanager))
  (bind _returnvalue_4 (Math|Rotator|FindLookatRotation _returnvalue_2 _returnvalue_3))
  (bind _newvar_0 (Variables|Default|GetNewVar_0)
    (:then
      (Default|SetValue _newvar_0 (/ (Variables|/Game/Duel/Blueprints/Characters/CH_Character.CH_Character_C|GetHP (Variables|Default|GetOwnerPlayer)) 1e+02))
      (Transformation|SetWorldLocation (Variables|Default|GetWidget) (+ (Transformation|GetWorldLocation (Variables|/Game/Duel/Blueprints/Characters/ThirdPersonCharacter.ThirdPersonCharacter_C|GetSkeletalMesh (Variables|Default|GetOwnerPlayer))) "0, 0,195.000000") false false)
      (Transformation|SetWorldRotation _widget (Math|Rotator|MakeRotator 0.0 (.pitch _returnvalue_4) (.yaw _returnvalue_4)) false false)
      (Class|WidgetComponent|RequestRedraw (Variables|Default|GetWidget)))
    (:else)))

(event EventBeginPlay
  (bind _asch_vrcharacter_pvp (Utilities|Casting|CastToCH_VRCharacterPVP (Components|GetOwner)))
  (Variables|Default|SetOwnerPlayer _asch_vrcharacter_pvp)
  (bind _asui_hp (Utilities|Casting|CastToUI_HP (UserInterface|GetUserWidgetObject (Variables|Default|GetWidget))))
  (Variables|Default|SetNewVar_0 _asui_hp)
  (Utilities|Time|SetTimerbyEvent (delegate Custom|CustomTimer) 0.05 true))

(fn ConstructionScript)